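; Game mode that opens the mayor selection widget at BeginPlay and applies the effects of each mayor: Jack, Hazel or Count.
; Each mayor function passes its house card to CheckCards on the main HUD and sets the Mayor enum.
; Jack and Hazel also spawn their actors, Hazel lowers XPNeeded, and Count's spawn node is unconnected.
; A delay-driven calendar counter from minutes to years is present but never runs.
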(event EventBeginPlay
  (bind _returnvalue (UserInterface|CreateWidget "/Game/UI/W_MayorSelect.W_MayorSelect_C"))
  (UserInterface|Viewport|AddtoViewport _returnvalue 0))

(event EventTick
  (params (DeltaSeconds :type Float%20%28single-precision%29)))

(fn ConstructionScript)

(fn MayorJack
  (bind _foundwidgets (Widget|GetAllWidgetsOfClass "/Game/UI/W_MainHUD.W_MainHUD_C" true))
  (Default|CheckCards (Utilities|Array|Get(acopy) _foundwidgets) "jackHouse")
  (Game|SpawnActorfromClass "/Game/Characters/BP_Jack.BP_Jack_C" (Math|Transform|MakeTransform "0, 0, 0" "0, 0, 0" "1.000000,1.000000,1.000000") "Undefined" 0 0)
  (Development|PrintString "Jack")
  (Variables|Default|SetMayor "NewEnumerator1"))

(fn MayorHazel
  (bind _foundwidgets (Widget|GetAllWidgetsOfClass "/Game/UI/W_MainHUD.W_MainHUD_C" true))
  (Default|CheckCards (Utilities|Array|Get(acopy) _foundwidgets) "hazelHouse")
  (Game|SpawnActorfromClass "/Game/Characters/BP_Hazel.BP_Hazel_C" (Math|Transform|MakeTransform "0, 0, 0" "0, 0, 0" "1.000000,1.000000,1.000000") "Undefined" 0 0)
  (Development|PrintString "Hazel")
  (Variables|Default|SetMayor "NewEnumerator2")
  (bind _output_get (Variables|Default|SetXP_Needed (- (stale _output_get) 5))))

(fn MayorCount
  (bind _foundwidgets (Widget|GetAllWidgetsOfClass "/Game/UI/W_MainHUD.W_MainHUD_C" true))
  (Default|CheckCards (Utilities|Array|Get(acopy) _foundwidgets) "countHouse")
  (Development|PrintString "Count")
  (Variables|Default|SetMayor "NewEnumerator3"))