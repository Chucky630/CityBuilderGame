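; BP_CardFactory is a placeable factory building that opens its own HUD when edited.
; BeginPlay enables player input, and the EditPlacedItem function creates W_FactoryHUD, adds it to the viewport and returns false.
; An unconnected graph would, once Built, read CardFactory_CardDataTable rows and send each card's build data to W_MainHUD's FactoryCards, but it never runs.
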(event EventBeginPlay
  (|CallParentFunction)
  (Input|EnableInput (Game|GetPlayerController 0)))

(event Collision|EventActorBeginOverlap
  (params (OtherActor :type Actor%20Object%20Reference))
  (|CallParentFunction OtherActor) ; This node is disabled and will not be called.\nDrag off pins to build functionality.
)

(event EventTick
  (params (DeltaSeconds :type Float%20%28single-precision%29))
  (|CallParentFunction DeltaSeconds))

(fn ConstructionScript
  (|CallParentFunction))

(fn EditPlacedItem
  (bind _returnvalue (UserInterface|CreateWidget "/Game/UI/W_FactoryHUD.W_FactoryHUD_C"))
  (UserInterface|Viewport|AddtoViewport _returnvalue 0)
  (return false))