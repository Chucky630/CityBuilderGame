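; Placeable road piece for the building system that follows the cursor on a grid until left-clicked, with mouse-wheel rotation.
; While editable, the wheel also cycles meshes and four clickable arrows spawn adjoining BP_Road pieces, locking the current one.
; R toggles between moving and editing, and EditPlacedItem reopens a placed piece.
; Construction reads building data from a table, but the timed population growth event is empty.
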(event OnClicked(ArrowX)
  (params (TouchedComponent :type Primitive%20Component%20Object%20Reference) (ButtonPressed :type Key%20Structure))
  (bind _arrowx (Variables|Default|GetArrowX))
  (if (Variables|Default|GetEditable)
    (Game|SpawnActorfromClass "BP_Road_C" (Math|Transform|MakeTransform (Transformation|GetWorldLocation _arrowx) (Transformation|GetWorldRotation _arrowx) "1.000000,1.000000,1.000000") "Undefined" 0 0)
    (CallFunction|RoadPlaced)))

(event OnClicked(ArrowX-2)
  (params (TouchedComponent :type Primitive%20Component%20Object%20Reference) (ButtonPressed :type Key%20Structure))
  (bind _arrowx_2 (Variables|Default|GetArrowX-2))
  (if (Variables|Default|GetEditable)
    (Game|SpawnActorfromClass "BP_Road_C" (Math|Transform|MakeTransform (Transformation|GetWorldLocation _arrowx_2) (Transformation|GetWorldRotation _arrowx_2) "1.000000,1.000000,1.000000") "Undefined" 0 0)
    (CallFunction|RoadPlaced)))

(event OnClicked(ArrowY)
  (params (TouchedComponent :type Primitive%20Component%20Object%20Reference) (ButtonPressed :type Key%20Structure))
  (bind _arrowy (Variables|Default|GetArrowY))
  (if (Variables|Default|GetEditable)
    (Game|SpawnActorfromClass "BP_Road_C" (Math|Transform|MakeTransform (Transformation|GetWorldLocation _arrowy) (Transformation|GetWorldRotation _arrowy) "1.000000,1.000000,1.000000") "Undefined" 0 0)
    (CallFunction|RoadPlaced)))

(event OnClicked(ArrowY-2)
  (params (TouchedComponent :type Primitive%20Component%20Object%20Reference) (ButtonPressed :type Key%20Structure))
  (bind _arrowy_2 (Variables|Default|GetArrowY-2))
  (if (Variables|Default|GetEditable)
    (Game|SpawnActorfromClass "BP_Road_C" (Math|Transform|MakeTransform (Transformation|GetWorldLocation _arrowy_2) (Transformation|GetWorldRotation _arrowy_2) "1.000000,1.000000,1.000000") "Undefined" 0 0)
    (CallFunction|RoadPlaced)))

(event Custom|PopulationGrowth
  ;[1 1 1] Population gowth, depending on data from table
)

(event Custom|mouseFollow
  (bind _returnvalue (Game|GetPlayerController 0))
  (bind _object_types (Variables|Default|GetObject%20Types))
  (bind _hitresult (Class|PlayerController|GetHitResultUnderCursorforObjects _returnvalue _object_types true))
  (bind _location (Collision|BreakHitResult _hitresult))
  (bind (_x _y _z) (Math|Vector|BreakVector _location))
  (bind _returnvalue_2 (Math|Float|SnapToGrid(Float) _x 1e+02))
  (bind _returnvalue_3 (Math|Float|SnapToGrid(Float) _y 1e+02))
  ;[1 1 1] meshFollows mouse location, places mesh as location once clicked
  (if (not (Variables|Default|GetleftMouseClicked))
    (Transformation|SetActorLocation self (Math|Vector|MakeVector _returnvalue_2 _returnvalue_3 _z) false false)
    (Variables|Default|SetWorldLocation (Math|Vector|MakeVector _returnvalue_2 _returnvalue_3 _z))))

(event Custom|EditMode
  (bind _asbp_character (Utilities|Casting|CastToBP_Character (Game|GetPlayerCharacter 0)))
  (Variables|/Game/BP_Character.BP_Character_C|SetIsInEditMode _asbp_character true)
  (Utilities|Time|SetTimerbyEvent (delegate Custom|mouseFollow) 0.03 true))

(event Custom|RoadPlaced
  (bind _arrowx (Variables|Default|GetArrowX))
  (Variables|Default|SetEditable false)
  (Rendering|SetVisibility _arrowx false false)
  (Collision|SetCollisionEnabled _arrowx "NoCollision"))

(event EventBeginPlay
  ;[1 1 1] Run time, enables mouse input, sets the mesh to the chosen mesh
  (Input|EnableInput (Game|GetPlayerController 0))
  (CallFunction|EditMode))

(event EventTick
  (params (DeltaSeconds :type Float%20%28single-precision%29))
  (if (Variables|Default|GetEditable)
    (Components|StaticMesh|SetStaticMesh (Variables|Default|GetStaticMesh) (Utilities|Array|Get(acopy) (Variables|Default|GetStaticMeshChang) (Variables|Default|GetMeshSelect)))))

(event Input|MouseEvents|MouseWheelAxis
  (params (AxisValue :type Float%20%28single-precision%29))
  ;[1 1 1] Rotate Mesh
  (if (not (Variables|Default|GetleftMouseClicked))
    (Transformation|AddRelativeRotation (Variables|Default|GetStaticMesh) (Math|Rotator|MakeRotator 0.0 0.0 (* AxisValue 15.0)) false false)))

(event Input|MouseEvents|LeftMouseButton
  (params (Key :type Key%20Structure))
  ;[1 1 1] Disables input, sets mesh and material to building zone
  (:Pressed
    (Variables|Default|SetleftMouseClicked true)
    (bind _asbp_character (Utilities|Casting|CastToBP_Character (Game|GetPlayerCharacter 0)))
    (Variables|/Game/BP_Character.BP_Character_C|SetIsInEditMode _asbp_character false)
    (Collision|SetCollisionEnabled (Variables|Default|GetStaticMesh) "QueryAndPhysics")
    (CallFunction|RoadPlaced)
    (Input|DisableInput (Game|GetPlayerController 0))
    ;[1 1 1] Changes building to specific building, after build time is up
    (Variables|Default|SetBuilt true)
    ;[1 1 1] Run event Population Growth
    (if (Variables|Default|GetGive%20Population?)
      (Utilities|Time|SetTimerbyEvent (delegate Custom|PopulationGrowth) (Math|Conversions|ToFloat(Integer) (Variables|Default|GetGrowth%20Delay)) true))))

(event Input|MouseEvents|MouseWheelUp
  (params (Key :type Key%20Structure))
  (bind _staticmeshchang (Variables|Default|GetStaticMeshChang))
  (bind _returnvalue (Utilities|Array|Length _staticmeshchang))
  (:Pressed
    (if (Variables|Default|GetEditable)
      (Utilities|FlowControl|Delay 0.03)
      (bind _output_get (Variables|Default|SetMeshSelect (Math|Integer|Clamp(Integer) (+ (stale _output_get) 1) 0 _returnvalue)))
      (if (>= (Variables|Default|GetMeshSelect) _returnvalue)
        (Variables|Default|SetMeshSelect 0)))))

(event Input|MouseEvents|MouseWheelDown
  (params (Key :type Key%20Structure))
  (bind _staticmeshchang (Variables|Default|GetStaticMeshChang))
  (bind _returnvalue (Utilities|Array|Length _staticmeshchang))
  (:Pressed
    (if (Variables|Default|GetEditable)
      (Utilities|FlowControl|Delay 0.03)
      (bind _output_get (Variables|Default|SetMeshSelect (Math|Integer|Clamp(Integer) (- (stale _output_get) 1) -1 _returnvalue)))
      (if (< (Variables|Default|GetMeshSelect) 0)
        (Variables|Default|SetMeshSelect (- _returnvalue 1))))))

(event Input|KeyboardEvents|R
  (params (Key :type Key%20Structure))
  (bind _staticmesh (Variables|Default|GetStaticMesh))
  (:Pressed
    (Utilities|FlowControl|FlipFlop
      (:A
        (Variables|Default|SetEditable false)
        (Variables|Default|SetleftMouseClicked false)
        (Collision|SetCollisionEnabled _staticmesh "NoCollision"))
      (:B
        (Variables|Default|SetEditable true)
        (Variables|Default|SetleftMouseClicked true)
        (Collision|SetCollisionEnabled _staticmesh "QueryAndPhysics")))))

(fn ConstructionScript
  (bind _returnvalue (Utilities|GetDataTableRow "/Game/Buildings/BaseBuilds/Buildings_dataTable.Buildings_dataTable" (Variables|Default|GetRow%20Name))
    (:then
      (Variables|Default|SetBuild%20Time (.buildtime _returnvalue))
      (Variables|Default|SetDesiredMesh (.mesh _returnvalue))
      (Variables|Default|SetGive%20Population? (.giveincume? _returnvalue))
      (Variables|Default|SetPopulation%20Growth (.incume _returnvalue))
      (Variables|Default|SetGrowth%20Delay (.incumedelay _returnvalue)))))

(fn EditPlacedItem
  (bind _arrowx (Variables|Default|GetArrowX))
  (Rendering|SetVisibility _arrowx true false)
  (Collision|SetCollisionEnabled _arrowx "QueryAndPhysics")
  (Variables|Default|SetEditable true)
  (Input|EnableInput (Game|GetPlayerController 0)))