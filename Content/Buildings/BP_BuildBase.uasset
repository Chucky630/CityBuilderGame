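; Base actor for a placeable city-builder building, configured from a data table row and adjusted by the chosen Mayor.
; A preview mesh follows the cursor on a grid and rotates by wheel; clicking shows a construction mesh, then after the build delay swaps meshes, spawns a character and grants cards.
; An optional timer flags income behind a camera-facing widget.
; EditPlacedItem re-enters placement in build mode, otherwise collects income or opens the building UI.
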(event Custom|IncumeGrowth
  ;[1 1 1] Population gowth, depending on data from table
  (if (>= (Variables|Default|GetDelayCounter) (Variables|Default|GetIncume%20Delay))
    (Development|SetHiddeninGame (Variables|Default|GetWidget) false false)
    (Variables|Default|SetIncumeAvailable true)
    (else
      (bind _output_get (Variables|Default|SetDelayCounter (+ (stale _output_get) 1))))))

(event Custom|mouseFollow
  (bind _returnvalue (Game|GetPlayerController 0))
  (bind _object_types (Variables|Default|GetObject%20Types))
  (bind _hitresult (Class|PlayerController|GetHitResultUnderCursorforObjects _returnvalue _object_types true))
  (bind _location (Collision|BreakHitResult _hitresult))
  (bind (_x _y _z) (Math|Vector|BreakVector _location))
  ;[1 1 1] meshFollows mouse location, places mesh as location once clicked
  (if (not (Variables|Default|GetleftMouseClicked))
    (Transformation|SetActorLocation self (Math|Vector|MakeVector (Math|Float|SnapToGrid(Float) _x 1e+02) (Math|Float|SnapToGrid(Float) _y 1e+02) _z) false false)))

(event Custom|EditMode
  (bind _asbp_character (Utilities|Casting|CastToBP_Character (Game|GetPlayerCharacter 0)))
  (Variables|/Game/BP_Character.BP_Character_C|SetIsInEditMode _asbp_character true)
  (Utilities|Time|SetTimerbyEvent (delegate Custom|mouseFollow) 0.03 true))

(event Custom|OpenUI
  (bind _returnvalue (Utilities|GetDataTableRow "/Game/Buildings/BaseBuilds/Buildings_dataTable.Buildings_dataTable" (Variables|Default|GetRow%20Name))
    (:then
      (bind _returnvalue_2 (UserInterface|CreateWidget "/Game/UI/W_BuildingUI.W_BuildingUI_C" 0 (.buildingname _returnvalue) (.incume _returnvalue) (.xp _returnvalue) (.incumedelay _returnvalue) (Variables|Default|GetDelayCounter) (.bp_class _returnvalue)))
      (UserInterface|Viewport|AddtoViewport _returnvalue_2 0)
      (Variables|Default|SetUIOpen true)
      (Utilities|Time|SetTimerbyEvent (delegate Custom|RefreshUI) 0.01 true))))

(event Custom|RefreshUI
  (if (Variables|Default|GetUIOpen)
    (bind _foundwidgets (Widget|GetAllWidgetsOfClass "/Game/UI/W_BuildingUI.W_BuildingUI_C" true))
    (Variables|/Game/UI/W_BuildingUI.W_BuildingUI_C|SetDelayCounter (Utilities|Array|Get(acopy) _foundwidgets) (Variables|Default|GetDelayCounter))))

(event EventBeginPlay
  (bind _staticmesh (Variables|Default|GetStaticMesh))
  ;[1 1 1] Run time, enables mouse input, sets the mesh to the chosen mesh
  (Input|EnableInput (Game|GetPlayerController 0))
  (bind _asbp_gamemode (Utilities|Casting|CastToBP_Gamemode (Game|GetGameMode)))
  (switch Utilities|FlowControl|Switch|SwitchonEnum_Mayor (Variables|/Game/BP_Gamemode.BP_Gamemode_C|GetMayor _asbp_gamemode)
    (:NewEnumerator1
      (bind _output_get (Variables|Default|SetBuild%20Time (- (stale _output_get) 1))))
    (:NewEnumerator2
      (bind _output_get_2 (Variables|Default|SetIncume%20Growth (+ (stale _output_get_2) 2))))
    (:NewEnumerator3
      _))
  (Components|StaticMesh|SetStaticMesh _staticmesh (Variables|Default|GetDesiredMesh))
  (for _index (range 0 10)
    (Rendering|Material|SetMaterial _staticmesh _index "/Game/Material/M_Preview.M_Preview")
    (CallFunction|EditMode)))

(event EventTick
  (params (DeltaSeconds :type Float%20%28single-precision%29))
  (Transformation|SetWorldRotation (Variables|Default|GetWidget) (Math|Conversions|RotationFromXVector (Math|Vector|Normalize (* (- (Camera|GetCameraLocation (Game|GetPlayerCameraManager 0)) (Transformation|GetWorldLocation (Variables|Default|GetWidget))) "1.000000,1.000000, 0"))) false false))

(event Input|MouseEvents|MouseWheelAxis
  (params (AxisValue :type Float%20%28single-precision%29))
  ;[1 1 1] Rotate Mesh
  (Transformation|AddRelativeRotation (Variables|Default|GetStaticMesh) (Math|Rotator|MakeRotator 0.0 0.0 (* AxisValue 15.0)) false false))

(event Input|MouseEvents|LeftMouseButton
  (params (Key :type Key%20Structure :default "None"))
  (bind _staticmesh (Variables|Default|GetStaticMesh))
  (:Pressed
    (if (Variables|Default|GetMoved?)
      (for _index (range 0 10)
        (Rendering|Material|SetMaterial (Variables|Default|GetStaticMesh) _index 0)
        (CallFunction|EditMode)
        (Variables|Default|SetleftMouseClicked true)
        (bind _asbp_character (Utilities|Casting|CastToBP_Character (Game|GetPlayerCharacter 0)))
        (Variables|/Game/BP_Character.BP_Character_C|SetIsInEditMode _asbp_character false)
        (Input|DisableInput (Game|GetPlayerController 0))
        (bind _asbp_gamemode (Utilities|Casting|CastToBP_Gamemode (Game|GetGameMode)))
        (Variables|/Game/BP_Gamemode.BP_Gamemode_C|SetBuildMode _asbp_gamemode true))
      (else
        ;[1 1 1] Disables input, sets mesh and material to building zone
        (Variables|Default|SetleftMouseClicked true)
        (bind _asbp_character_2 (Utilities|Casting|CastToBP_Character (Game|GetPlayerCharacter 0)))
        (Variables|/Game/BP_Character.BP_Character_C|SetIsInEditMode _asbp_character_2 false)
        (Input|DisableInput (Game|GetPlayerController 0))
        (Components|StaticMesh|SetStaticMesh _staticmesh "/Game/Buildings/Models/TempBuilding.TempBuilding")
        (for _index_2 (range 0 10)
          (Rendering|Material|SetMaterial _staticmesh _index_2 0)
          ;[1 1 1] Changes building to specific building, after build time is up
          (Utilities|FlowControl|Delay (Math|Conversions|ToFloat(Integer) (Variables|Default|GetBuild%20Time)))
          (Components|StaticMesh|SetStaticMesh (Variables|Default|GetStaticMesh) (Variables|Default|GetDesiredMesh))
          (Variables|Default|SetBuilt true)
          ;[1 1 1] Character being Spawned
          (Game|SpawnActorfromClass (Variables|Default|GetCharacter) (Math|Transform|MakeTransform "0, 0, 0" "0, 0, 0" "1.000000,1.000000,1.000000") "Undefined" 0 0)
          ;[1 1 1] Run event Population Growth
          (if (Variables|Default|GetGive%20Incume?)
            (Utilities|Time|SetTimerbyEvent (delegate Custom|IncumeGrowth) 1.0 true))
          ;[1 1 1] give player card by names in array
          (bind _foundwidgets (Widget|GetAllWidgetsOfClass "/Game/UI/W_MainHUD.W_MainHUD_C" true))
          (for _array_element (Variables|Default|GetRow%20NameGive)
            (Default|CheckCards (Utilities|Array|Get(acopy) _foundwidgets) _array_element)))))))

(fn ConstructionScript
  (bind _returnvalue (Utilities|GetDataTableRow "/Game/Buildings/BaseBuilds/Buildings_dataTable.Buildings_dataTable" (Variables|Default|GetRow%20Name))
    (:then
      (Variables|Default|SetBuild%20Time (.buildtime _returnvalue))
      (Variables|Default|SetDesiredMesh (.mesh _returnvalue))
      (Variables|Default|SetGive%20Incume? (.giveincume? _returnvalue))
      (Variables|Default|SetIncume%20Growth (.incume _returnvalue))
      (Variables|Default|SetIncume%20Delay (.incumedelay _returnvalue))
      (Variables|Default|SetXP (.xp _returnvalue)))))

(fn TaskBegin)

(fn EditPlacedItem
  (bind _asbp_gamemode (Utilities|Casting|CastToBP_Gamemode (Game|GetGameMode)))
  (if (Variables|/Game/BP_Gamemode.BP_Gamemode_C|GetBuildMode _asbp_gamemode)
    (for _index (range 0 10)
      (Rendering|Material|SetMaterial (Variables|Default|GetStaticMesh) _index "/Game/Material/M_Preview.M_Preview")
      (CallFunction|EditMode)
      (Variables|Default|SetleftMouseClicked false)
      (bind _asbp_character (Utilities|Casting|CastToBP_Character (Game|GetPlayerCharacter 0)))
      (Variables|/Game/BP_Character.BP_Character_C|SetIsInEditMode _asbp_character true)
      (Input|EnableInput (Game|GetPlayerController 0))
      (Variables|Default|SetMoved? true))
    (elif (Variables|Default|GetIncumeAvailable)
      (bind _asbp_gamemode_2 (Utilities|Casting|CastToBP_Gamemode (Game|GetGameMode)))
      (bind _output_get (Variables|/Game/BP_Gamemode.BP_Gamemode_C|SetPoints _asbp_gamemode_2 (+ (stale _output_get) (Variables|Default|GetIncume%20Growth))))
      (bind _output_get_2 (Variables|/Game/BP_Gamemode.BP_Gamemode_C|SetXP _asbp_gamemode_2 (+ (stale _output_get_2) (Variables|Default|GetXP))))
      (Variables|Default|SetDelayCounter 0)
      (Development|SetHiddeninGame (Variables|Default|GetWidget) true false)
      (Variables|Default|SetIncumeAvailable false)
      (elif (not (Variables|Default|GetUIOpen))
        (CallFunction|OpenUI)))))