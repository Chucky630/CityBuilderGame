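; BP_TownRubish is a town rubbish building Blueprint configured from the Buildings data table.
; Its Construction Script looks up RowName and copies build time, mesh and the income fields, which feed its population-growth settings.
; EditPlacedItem always returns false.
; An unconnected branch for CardFactory table data, with a debug print and population growth switched off, never runs.
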(fn ConstructionScript
  (bind _returnvalue (Utilities|GetDataTableRow "/Game/Buildings/BaseBuilds/Buildings_dataTable.Buildings_dataTable" (Variables|Default|GetRow%20Name))
    (:then
      (Variables|Default|SetBuild%20Time (.buildtime _returnvalue))
      (Variables|Default|SetDesiredMesh (.mesh _returnvalue))
      (Variables|Default|SetGive%20Population? (.giveincume? _returnvalue))
      (Variables|Default|SetPopulation%20Growth (.incume _returnvalue))
      (Variables|Default|SetGrowth%20Delay (.incumedelay _returnvalue)))))

(fn EditPlacedItem
  (return false))